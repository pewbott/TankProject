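; BP_EndSphere is a level goal actor that ends the level when a BP_Tank hits its static mesh.
; Tick feeds a 0.1-second Delay that increments LiveTimer, giving an approximate elapsed time since BeginPlay.
; On the hit, ShowResults passes that time to a WBP_EndLevel widget, pauses the game, destroys the sphere and shows the mouse cursor.
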(event OnComponentHit(StaticMesh)
  (params (HitComponent :type Primitive%20Component%20Object%20Reference) (OtherActor :type Actor%20Object%20Reference) (OtherComp :type Primitive%20Component%20Object%20Reference) (NormalImpulse :type Vector :default "0, 0, 0") (Hit :type Hit%20Result%20Structure%20%28by%20ref%29))
  (Utilities|Casting|CastToBP_Tank OtherActor)
  (CallFunction|ShowResults))

(event EventBeginPlay
  (Variables|Default|SetLive%20Timer 0.0))

(event Collision|EventActorBeginOverlap
  (params (OtherActor :type Actor%20Object%20Reference)))

(event EventTick
  (params (DeltaSeconds :type Float%20%28single-precision%29))
  (Utilities|FlowControl|Delay 0.1)
  (Variables|Default|SetLive%20Timer (+ (Variables|Default|GetLive%20Timer) 0.1)))

(fn ConstructionScript)

(fn ShowResults
  (bind _returnvalue (UserInterface|CreateWidget "/Game/Blueprints/UI/WBP_EndLevel.WBP_EndLevel_C"))
  (Variables|/Game/Blueprints/UI/WBP_EndLevel.WBP_EndLevel_C|SetTimer%20float _returnvalue (Variables|Default|GetLive%20Timer))
  (UserInterface|Viewport|AddtoViewport _returnvalue 0)
  (Game|SetGamePaused true)
  (Actor|DestroyActor)
  (Variables|/Script/Engine.PlayerController|SetbShowMouseCursor (Game|GetPlayerController 0) true))