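; A destructible blocking box that loses one Health per bullet hit and shows its remaining Health through color.
; BeginPlay creates a dynamic instance of M_BlockingBox on the mesh and tints it for the starting Health.
; Box component hits from BP_Bullet call GetDamage, which decrements Health, then either recolors the box through the ColorParam vector parameter or destroys it at zero.
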(event OnComponentHit(Box)
  (params (HitComponent :type Primitive%20Component%20Object%20Reference) (OtherActor :type Actor%20Object%20Reference) (OtherComp :type Primitive%20Component%20Object%20Reference) (NormalImpulse :type Vector :default "0, 0, 0") (Hit :type Hit%20Result%20Structure%20%28by%20ref%29))
  (Utilities|Casting|CastToBP_Bullet OtherActor)
  (CallFunction|GetDamage))

(event EventBeginPlay
  (CallFunction|CreateDynamicMaterial)
  (CallFunction|ChangeMaterialColor (Variables|Health|GetHealth)))

(event Collision|EventActorBeginOverlap
  (params (OtherActor :type Actor%20Object%20Reference)))

(event EventTick
  (params (DeltaSeconds :type Float%20%28single-precision%29)))

(fn ConstructionScript)

(fn GetDamage
  (bind _health (Variables|Health|GetHealth))
  (bind _result (Math|Integer|DecrementInt _health)
    (:%20%20
      (switch int _result
        (:0
          (Actor|DestroyActor))
        (:1
          (CallFunction|ChangeMaterialColor _health))
        (:2
          (CallFunction|ChangeMaterialColor _health))))))

(fn CreateDynamicMaterial
  (bind _boxmesh (Variables|Default|GetBoxMesh))
  (bind _returnvalue (Rendering|Material|CreateDynamicMaterialInstance _boxmesh 0 "/Game/Materials/GameplayObjects/BlockingBoxes/M_BlockingBox.M_BlockingBox" "None" :!class /Script/Engine.PrimitiveComponent))
  (Rendering|Material|SetMaterial _boxmesh 0 _returnvalue))

(fn ChangeMaterialColor
  (params (value :type Integer))
  (bind _boxmesh (Variables|Default|GetBoxMesh))
  (switch int value
    (:0
      (Rendering|Material|SetVectorParameterValueonMaterials _boxmesh "ColorParam" "1.000000,1.000000,1.000000"))
    (:1
      (Rendering|Material|SetVectorParameterValueonMaterials _boxmesh "ColorParam" "0.000000,1.000000,0.000000"))
    (:2
      (Rendering|Material|SetVectorParameterValueonMaterials _boxmesh "ColorParam" "0.000000,0.000000,1.000000"))
    (:3
      (Rendering|Material|SetVectorParameterValueonMaterials _boxmesh "ColorParam" "1.000000,0.000000,0.000000"))))